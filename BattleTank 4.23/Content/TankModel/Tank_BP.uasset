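; Player-controllable tank Blueprint that wires input to its aiming and movement components.
; On BeginPlay it hands the barrel and turret to TankAiming and both tracks to TankMovement.
; Camera axes rotate an azimuth gimbal for yaw and the spring arm for pitch, keeping the two rotations on separate components.
; Firing input calls TankAiming, while move and turn axes pass intents to TankMovement.
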(event EventBeginPlay
  (Class|TankAimingComponent|Initialise (Variables|Default|GetTank%20Aiming) (Variables|Default|GetTankBarrel) (Variables|Default|GetTankTurret))
  (Class|TankMovementComponent|Initialise (Variables|Default|GetTank%20Movement) (Variables|Default|GetLeftTrack) (Variables|Default|GetRightTrack)))

(event Input|ActionEvents|InputActionFiring
  (params (Key :type Key%20Structure))
  ;[1 1 1] Firing input
  (:Pressed
    (Class|TankAimingComponent|Fire (Variables|Default|GetTank%20Aiming))))

(event Input|AxisEvents|InputAxisAimAzimuth
  (params (AxisValue :type Float%20%28single-precision%29))
  ;[1 1 1] Camera Input Binding
  (Transformation|AddLocalRotation (Variables|Default|GetAzimuth%20Gimble) (Math|Rotator|MakeRotator 0.0 0.0 AxisValue) false false))

(event Input|AxisEvents|InputAxisAimElevation
  (params (AxisValue :type Float%20%28single-precision%29))
  ;[1 1 1] Camera Input Binding
  (Transformation|AddLocalRotation (Variables|Default|GetSpringArm) (Math|Rotator|MakeRotator 0.0 AxisValue 0.0) false false))

(event Input|AxisEvents|InputAxisMoveAxial
  (params (AxisValue :type Float%20%28single-precision%29))
  ;[1 1 1] Moving input
  (Class|TankMovementComponent|IntendMoveForward (Variables|Default|GetTank%20Movement) AxisValue))

(event Input|AxisEvents|InputAxisTurn
  (params (AxisValue :type Float%20%28single-precision%29))
  ;[1 1 1] Moving input
  (Class|TankMovementComponent|IntendTurn (Variables|Default|GetTank%20Movement) AxisValue))

(fn ConstructionScript)